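; BP_Cable is a cable actor that links two target objects through its UmbilicalCable component.
; A custom event named 1234 passes both targets' root components as start and end points, then enables actor tick.
; Each tick calls UpdateCable on the component.
; A conditional delayed-update branch and a spare update call are left unconnected.
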(event `1234`
  (params (`目标` :type "Actor Object Reference") (`目标2` :type "Actor Object Reference"))
  (`UmbilicalCableComponent.SetTargetPoint` (`self.UmbilicalCable`) (`Actor.RootComponent` `目标`) (`Actor.RootComponent` `目标2`))
  (`self.SetActorTickEnabled` true))

(event `self.ReceiveTick`
  (params (DeltaSeconds :type "Float (single-precision)"))
  (`UmbilicalCableComponent.UpdateCable` (`self.UmbilicalCable`)))

(fn `UserConstructionScript`)